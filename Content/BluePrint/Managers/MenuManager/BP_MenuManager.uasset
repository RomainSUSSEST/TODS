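; Menu manager actor that owns the main menu canvas widget and drives the game's menu screens.
; It creates the canvas on BeginPlay, binds its button events and relays them, plus the Pause input, as its own events.
; Parent game-state overrides show the main, pause, game over or victory panel with cursor and UI-only input.
; Play, resume and play-again states call ShowPanel without a panel, hide the cursor and restore game-only input.
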(event Collision|EventActorBeginOverlap
  (params (OtherActor :type Actor%20Object%20Reference)))

(event EventTick
  (params (DeltaSeconds :type Float%20%28single-precision%29)))

(event EventBeginPlay
  ;[1 1 1] Initialisation Variable
  (bind _returnvalue (UserInterface|CreateWidget "/Game/WidgetBP/MainMenuCanvas_Widget.MainMenuCanvas_Widget_C" (Game|GetPlayerController 0)))
  (Variables|Default|SetCanvasWidget _returnvalue)
  (|CallParentFunction)
  (UserInterface|Viewport|AddtoViewport _returnvalue 0))

(event Input|ActionEvents|InputActionPause
  (params (Key :type Key%20Structure))
  ;[1 1 1] Escape Button Pressed
  (:Pressed
    (Default|CallEscapeButtonHasBeenPressedEvent)))

(fn ConstructionScript)

(fn SubscribeEvents
  (bind _canvaswidget (Variables|Default|GetCanvasWidget))
  ;[1 1 1] OnClick Button Event
  (|CallParentFunction)
  (EventDispatchers|BindEventtoExitButtonHasBeenClicked _canvaswidget (EventDispatchers|CreateEvent :!event CallExitButtonClickedEvent))
  (EventDispatchers|BindEventtoPlayButtonHasBeenClicked _canvaswidget (EventDispatchers|CreateEvent :!event CallPlayButtonClickedEvent))
  (EventDispatchers|BindEventtoResumeButtonHasBeenClicked _canvaswidget (EventDispatchers|CreateEvent :!event CallResumeButtonClickedEvent))
  (EventDispatchers|BindEventtoMenuButtonHasBeenClicked _canvaswidget (EventDispatchers|CreateEvent :!event CallMenuButtonClickedEvent))
  (EventDispatchers|BindEventtoRetryButtonHasBeenClicked _canvaswidget (EventDispatchers|CreateEvent :!event CallRetryButtonClickedClickedEvent))
  (EventDispatchers|BindEventtoQuit1ButtonHasBeenClicked _canvaswidget (EventDispatchers|CreateEvent :!event CallQuit1ButtonClickedEvent))
  (EventDispatchers|BindEventtoRestartButtonHasBeenClicked _canvaswidget (EventDispatchers|CreateEvent :!event CallRestartButtonHasBeenClickedEvent))
  (EventDispatchers|BindEventtoExit1ButtonHasBeenClicked _canvaswidget (EventDispatchers|CreateEvent :!event CallExit1ButtonButtonHasBeenClickedEvent))
  (Input|EnableInput (Game|GetPlayerController 0)))

(fn CallExitButtonClickedEvent
  (Default|CallExitButtonHasBeenClickedEvent))

(fn CallPlayButtonClickedEvent
  (Default|CallPlayButtonHasBeenClickedEvent))

(fn GameMainMenu
  (bind _returnvalue (Game|GetPlayerController 0))
  (bind _canvaswidget (Variables|Default|GetCanvasWidget))
  (|CallParentFunction)
  (Default|ShowPanel _canvaswidget (Variables|/Game/WidgetBP/MainMenuCanvas_Widget.MainMenuCanvas_Widget_C|GetPanel_MainMenu _canvaswidget))
  (Variables|/Script/Engine.PlayerController|SetbShowMouseCursor _returnvalue true)
  (Input|SetInputModeUIOnly _returnvalue (Variables|Default|GetCanvasWidget) "DoNotLock"))

(fn GamePlay
  (bind _returnvalue (Game|GetPlayerController 0))
  (|CallParentFunction)
  (Default|ShowPanel (Variables|Default|GetCanvasWidget))
  (Variables|/Script/Engine.PlayerController|SetbShowMouseCursor _returnvalue false)
  (Input|SetInputModeGameOnly _returnvalue))

(fn CallResumeButtonClickedEvent
  (Default|CallResumeButtonHasBeenClickedEvent))

(fn CallMenuButtonClickedEvent
  (Default|CallMenuButtonHasBeenClickedEvent))

(fn GamePause
  (bind _returnvalue (Game|GetPlayerController 0))
  (bind _canvaswidget (Variables|Default|GetCanvasWidget))
  (|CallParentFunction)
  (Default|ShowPanel _canvaswidget (Variables|/Game/WidgetBP/MainMenuCanvas_Widget.MainMenuCanvas_Widget_C|GetPanel_PauseMenu _canvaswidget))
  (Variables|/Script/Engine.PlayerController|SetbShowMouseCursor _returnvalue true)
  (Input|SetInputModeUIOnly _returnvalue (Variables|Default|GetCanvasWidget) "DoNotLock"))

(fn GameResume
  (bind _returnvalue (Game|GetPlayerController 0))
  (|CallParentFunction)
  (Default|ShowPanel (Variables|Default|GetCanvasWidget))
  (Variables|/Script/Engine.PlayerController|SetbShowMouseCursor _returnvalue false)
  (Input|SetInputModeGameOnly _returnvalue))

(fn GameOver
  (bind _returnvalue (Game|GetPlayerController 0))
  (bind _canvaswidget (Variables|Default|GetCanvasWidget))
  (|CallParentFunction)
  (Default|ShowPanel _canvaswidget (Variables|/Game/WidgetBP/MainMenuCanvas_Widget.MainMenuCanvas_Widget_C|GetPanel_GameOver _canvaswidget))
  (Variables|/Script/Engine.PlayerController|SetbShowMouseCursor _returnvalue true)
  (Input|SetInputModeUIOnly _returnvalue (Variables|Default|GetCanvasWidget) "DoNotLock"))

(fn GameVictory
  (bind _returnvalue (Game|GetPlayerController 0))
  (bind _canvaswidget (Variables|Default|GetCanvasWidget))
  (|CallParentFunction)
  (Default|ShowPanel _canvaswidget (Variables|/Game/WidgetBP/MainMenuCanvas_Widget.MainMenuCanvas_Widget_C|GetPanel_GameVictory _canvaswidget))
  (Variables|/Script/Engine.PlayerController|SetbShowMouseCursor _returnvalue true)
  (Input|SetInputModeUIOnly _returnvalue (Variables|Default|GetCanvasWidget) "DoNotLock"))

(fn CallRetryButtonClickedClickedEvent
  (Default|CallRetryButtonHasBeendClickedEvent))

(fn CallQuit1ButtonClickedEvent
  (Default|CallQuit1ButtonHasBeenClickedEvent))

(fn CallRestartButtonHasBeenClickedEvent
  (Default|CallRestartButtonHasBeenClickedEvent))

(fn CallExit1ButtonButtonHasBeenClickedEvent
  (Default|CallExit1ButtonHasBeenClicked))

(fn GamePlayAgain
  (bind _returnvalue (Game|GetPlayerController 0))
  (|CallParentFunction)
  (Default|ShowPanel (Variables|Default|GetCanvasWidget))
  (Variables|/Script/Engine.PlayerController|SetbShowMouseCursor _returnvalue false)
  (Input|SetInputModeGameOnly _returnvalue))
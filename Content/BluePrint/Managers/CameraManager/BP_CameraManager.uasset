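; BP_CameraManager switches player 0's view to the menu camera when the game enters the main menu or options.
; It overrides game-state functions from its parent, calling the parent version first, then using SetViewTargetWithBlend to target MenuCamera with no blend time specified.
; The GamePlay and GameResume overrides only call the parent, so this Blueprint itself never switches the view back from MenuCamera.
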(event Collision|EventActorBeginOverlap
  (params (OtherActor :type Actor%20Object%20Reference)))

(event EventTick
  (params (DeltaSeconds :type Float%20%28single-precision%29)))

(fn ConstructionScript)

(fn GamePlay
  (|CallParentFunction))

(fn GameOptions
  (|CallParentFunction)
  (Game|Player|SetViewTargetwithBlend (Game|GetPlayerController 0) (Variables|Default|GetMenuCamera) 0.0 "VTBlend_Linear" 0.0 false))

(fn GameResume
  (|CallParentFunction))

(fn GameMainMenu
  (|CallParentFunction)
  (Game|Player|SetViewTargetwithBlend (Game|GetPlayerController 0) (Variables|Default|GetMenuCamera) 0.0 "VTBlend_Linear" 0.0 false))
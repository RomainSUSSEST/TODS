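; BP_ManagerReferences is an actor that acts as a central holder of references to the game, menu, level and music manager instances.
; Getter functions expose each stored manager to other code.
; AllManagerIsReady queries IsReady on all four managers and returns true only when every one reports ready.
; The event graph and construction script are empty, so nothing here assigns the references.
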(event EventBeginPlay)

(event Collision|EventActorBeginOverlap
  (params (OtherActor :type Actor%20Object%20Reference)))

(event EventTick
  (params (DeltaSeconds :type Float%20%28single-precision%29)))

(fn ConstructionScript)

(fn GetGameManagerInstance
  (return (Variables|Default|GetGameManager)))

(fn GetMenuManagerInstance
  (return (Variables|Default|GetMenuManager)))

(fn AllManagerIsReady
  (bind _ready (Default|IsReady (Variables|Default|GetGameManager)))
  (bind _ready_2 (Default|IsReady (Variables|Default|GetMenuManager)))
  (bind _ready_3 (Default|IsReady (Variables|Default|GetLevelManager)))
  (bind _ready_4 (Default|IsReady (Variables|Default|GetMusicManager)))
  (return (Math|Boolean|ANDBoolean _ready_3 _ready_2 _ready _ready_4)))

(fn GetLevelManagerInstance
  (return (Variables|Default|GetLevelManager)))

(fn GetMusicManager
  (return (Variables|Default|GetMusicManager)))
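; Game manager Blueprint that owns the high-level game state: main menu, options, play, pause, resume and quit.
; On BeginPlay it polls with a zero-length Delay until all managers report ready, then subscribes to MenuManager button and Escape events and opens the main menu.
; Each state function sets GameState and global time dilation, zero when paused, then calls its own event dispatcher to broadcast the change.
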(event Collision|EventActorBeginOverlap
  (params (OtherActor :type Actor%20Object%20Reference)))

(event EventTick
  (params (DeltaSeconds :type Float%20%28single-precision%29)))

(event EventBeginPlay
  ;[1 1 1] Initialisation
  (|CallParentFunction)
  (bind _managerreferences (CallFunction|GetManagerReferences))
  (bind _value (Default|AllManagerIsReady _managerreferences :!label _label))
  (if _value
    (CallFunction|SubscribeEvent)
    (CallFunction|MainMenu)
    (else
      (Utilities|FlowControl|Delay 0.0)
      (goto _label))))

(fn ConstructionScript)

(fn MainMenu
  (Utilities|Time|SetGlobalTimeDilation 1.0)
  (Variables|Default|SetGameState "NewEnumerator0")
  (Default|CallGameMainMenuEvent0))

(fn OptionsMenu
  (Utilities|Time|SetGlobalTimeDilation 1.0)
  (Variables|Default|SetGameState "NewEnumerator0")
  (Default|CallGameOptionsMenuEvent0))

(fn Play
  (Utilities|Time|SetGlobalTimeDilation 1.0)
  (Variables|Default|SetGameState "NewEnumerator1")
  (Default|CallGamePlayEvent0))

(fn Pause
  (Utilities|Time|SetGlobalTimeDilation 0.0)
  (Variables|Default|SetGameState "NewEnumerator2")
  (Default|CallGamePauseEvent0))

(fn Resume
  (Utilities|Time|SetGlobalTimeDilation 1.0)
  (Variables|Default|SetGameState "NewEnumerator1")
  (Default|CallGameResumeEvent0))

(fn SubscribeEvent
  ;[1 1 1] MenuManager Instance
  (bind _managerreferences (CallFunction|GetManagerReferences))
  (bind _menumanager (Default|GetMenuManagerInstance _managerreferences))
  ;[1 1 1] Onclick Event
  (EventDispatchers|BindEventtoPlayButtonHasBeenClickedEvent _menumanager (EventDispatchers|CreateEvent :!event Play))
  (EventDispatchers|BindEventtoOptionsButtonHasBeenClickedEvent _menumanager (EventDispatchers|CreateEvent :!event OptionsMenu))
  (EventDispatchers|BindEventtoExitButtonHasBeenClickedEvent _menumanager (EventDispatchers|CreateEvent :!event ExitGame))
  (EventDispatchers|BindEventtoResumeButtonHasBeenClickedEvent _menumanager (EventDispatchers|CreateEvent :!event Resume))
  (EventDispatchers|BindEventtoMenuButtonHasBeenClickedEvent _menumanager (EventDispatchers|CreateEvent :!event MainMenu))
  ;[1 1 1] Key Press
  (EventDispatchers|BindEventtoEscapeButtonHasBeenPressedEvent _menumanager (EventDispatchers|CreateEvent :!event Pause)))

(fn ExitGame
  (Game|QuitGame 0 "Quit" false))
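; Level manager that streams the game's world background and level sequence in and out as the game state changes.
; Game-state overrides raise its own events to initialize or unload; initialization loads the background, then the first entry of ListLevels.
; Level success swaps in the next level or triggers victory, and player death triggers game over.
; Delay loops poll for background load and player; the finish point is bound only during initialization.
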(event Custom|UnloadCurrentWorld
  ;[1 1 1] SubscribeEvents
  (Game|UnloadStreamLevel(byName) (Variables|Default|GetCurrentWorld) true))

(event Custom|UnloadCurrentLevel
  ;[1 1 1] SubscribeEvents
  (Game|UnloadStreamLevel(byName) (Variables|Default|GetCurrentLevelName) true))

(event Custom|PlayerDead
  ;[1 1 1] GameOverForCurrentLevel
  (Default|CallGameOverEvent))

(event Custom|InitializeGame
  ;[1 1 1] SubscribeEvents
  (Variables|Default|SetNextLevelIndex 0)
  ;[1 1 1] World1
  (bind _returnvalue (Class|LevelStreamingDynamic|LoadLevelInstance (Variables|Default|GetWorld1_Background) "0, 0, 0" "0, 0, 0"))
  (Variables|Default|SetCurrentWorld (Class|LevelStreaming|GetWorldAssetPackageFName _returnvalue))
  ;[1 1 1] Waiting
  (if (Class|LevelStreaming|IsLevelLoaded _returnvalue) :!label _label
    ;[1 1 1] Level1
    (bind _astods_player_controller (Utilities|Casting|CastToTodsPlayerController (Game|GetPlayerController 0)))
    (Default|SetCurrentPlayer _astods_player_controller)
    (bind _returnvalue_2 (Class|LevelStreamingDynamic|LoadLevelInstance (Utilities|Array|Get(acopy) (Variables|Default|GetListLevels) (Variables|Default|GetNextLevelIndex)) "0, 0, 0" "0, 0, 0"))
    (Variables|Default|SetCurrentLevelName (Class|LevelStreaming|GetWorldAssetPackageFName _returnvalue_2))
    (Math|Integer|IncrementInt (Variables|Default|GetNextLevelIndex)
      (:%20%20
        ;[1 1 1] GameOverForCurrentLevel
        (bind _astods_player_controller_2 (Utilities|Casting|CastToTodsPlayerController (Game|GetPlayerController 0)))
        (bind _player (Default|GetCurrentPlayer _astods_player_controller_2 :!label _label_2))
        (if (== _player 0)
          (Utilities|FlowControl|Delay 0.2)
          (goto _label_2)
          (else
            (EventDispatchers|BindEventtoPlayerDeadEvent _player (delegate Custom|PlayerDead))
            ;[1 1 1] Next Level
            (EventDispatchers|BindEventtoLevelSuccess (Variables|/Game/UnrealManager/TodsPlayerController.TodsPlayerController_C|GetCurrentFinishPoint _astods_player_controller_2) (delegate Custom|LevelSuccess))))))
    (else
      (Utilities|FlowControl|Delay 0.2)
      (goto _label))))

(event Custom|DeadPlayer2
  ;[1 1 1] GameOverForCurrentLevel
  (Default|CallGameOverEvent))

(event Custom|LevelSuccess
  ;[1 1 1] Next Level
  (Default|CallLevelSuccessEvent))

(event Custom|LoadNextlevel
  (bind _nextlevelindex (Variables|Default|GetNextLevelIndex))
  ;[1 1 1] SubscribeEvents
  (if (>= (Variables|Default|GetNextLevelIndex) (Utilities|Array|Length (Variables|Default|GetListLevels)))
    ;[1 1 1] GameVictory
    (Default|CallGameVictoryEvent)
    (else
      ;[1 1 1] LoadNextLevel
      (Default|CallUnloadCurrentLevelEventEvent)
      (bind _astods_player_controller (Utilities|Casting|CastToTodsPlayerController (Game|GetPlayerController 0)))
      (Default|SetCurrentPlayer _astods_player_controller)
      (bind _returnvalue (Class|LevelStreamingDynamic|LoadLevelInstance (Utilities|Array|Get(acopy) (Variables|Default|GetListLevels) _nextlevelindex) "0, 0, 0" "0, 0, 0"))
      (Variables|Default|SetCurrentLevelName (Class|LevelStreaming|GetWorldAssetPackageFName _returnvalue))
      (Math|Integer|IncrementInt _nextlevelindex
        (:%20%20
          ;[1 1 1] GameOverForCurrentLevel
          (bind _astods_player_controller_2 (Utilities|Casting|CastToTodsPlayerController (Game|GetPlayerController 0)))
          (bind _player (Default|GetCurrentPlayer _astods_player_controller_2 :!label _label))
          (if (== _player 0)
            (Utilities|FlowControl|Delay 0.2)
            (goto _label)
            (else
              (EventDispatchers|BindEventtoPlayerDeadEvent _player (delegate Custom|DeadPlayer2)))))))))

(event EventBeginPlay
  ;[1 1 1] SubscribeEvents
  (|CallParentFunction)
  (EventDispatchers|BindEventtoUnloadCurrentLevelEventEvent (delegate Custom|UnloadCurrentLevel))
  (EventDispatchers|BindEventtoUnloadCurrentWorldEvent (delegate Custom|UnloadCurrentWorld))
  (EventDispatchers|BindEventtoInitializeGameEvent (delegate Custom|InitializeGame))
  (EventDispatchers|BindEventtoLevelSuccessEvent (delegate Custom|LoadNextlevel)))

(fn ConstructionScript)

(fn GamePlay
  (|CallParentFunction)
  (Default|CallInitializeGameEvent))

(fn GameMainMenu
  (|CallParentFunction)
  (if (not (Utilities|Name|Equal(Name) (Variables|Default|GetCurrentLevelName) "None"))
    (Default|CallUnloadCurrentLevelEventEvent)
    (Default|CallUnloadCurrentWorldEvent)))

(fn GameOver
  (|CallParentFunction)
  (Default|CallUnloadCurrentLevelEventEvent)
  (Default|CallUnloadCurrentWorldEvent)
  (bind _astods_game_mode (Utilities|Casting|CastToTodsGameMode (Game|GetGameMode)))
  (Default|DestroyAllInstanciedObject _astods_game_mode))

(fn GameVictory
  (|CallParentFunction)
  (Default|CallUnloadCurrentLevelEventEvent)
  (Default|CallUnloadCurrentWorldEvent))

(fn GamePlayAgain
  (|CallParentFunction)
  (Default|CallUnloadCurrentLevelEventEvent)
  (Default|CallUnloadCurrentWorldEvent)
  (Default|CallInitializeGameEvent))
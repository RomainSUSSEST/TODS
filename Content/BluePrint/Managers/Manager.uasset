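; Base-style manager Blueprint that hooks into the GameManager's game-state events.
; On BeginPlay it gets the game manager instance through ManagerReferences, binds to its play, pause, options menu, resume and main menu events, then flags itself ready.
; Matching handler functions for each state are empty stubs.
; Getters expose the manager references and the ready flag.
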(event EventBeginPlay
  ;[1 1 1] Subscribe GameState Event
  (CallFunction|SubscribeEvents)
  (Variables|Default|SetReady true))

(event Collision|EventActorBeginOverlap
  (params (OtherActor :type Actor%20Object%20Reference)))

(event EventTick
  (params (DeltaSeconds :type Float%20%28single-precision%29)))

(fn ConstructionScript)

(fn GamePlay)

(fn GamePause)

(fn GameOptions)

(fn GameResume)

(fn GameMainMenu)

(fn GetManagerReferences
  (return (Variables|Default|GetManagerReferences)))

(fn SubscribeEvents
  ;[1 1 1] GameState Events
  (bind _gamemanager (Default|GetGameManagerInstance (Variables|Default|GetManagerReferences)))
  (EventDispatchers|BindEventtoGamePlayEvent0 _gamemanager (EventDispatchers|CreateEvent :!event GamePlay))
  (EventDispatchers|BindEventtoGamePauseEvent0 _gamemanager (EventDispatchers|CreateEvent :!event GamePause))
  (EventDispatchers|BindEventtoGameOptionsMenuEvent0 _gamemanager (EventDispatchers|CreateEvent :!event GameOptions))
  (EventDispatchers|BindEventtoGameResumeEvent0 _gamemanager (EventDispatchers|CreateEvent :!event GameResume))
  (EventDispatchers|BindEventtoGameMainMenuEvent0 _gamemanager (EventDispatchers|CreateEvent :!event GameMainMenu)))

(fn IsReady
  (return (Variables|Default|GetReady)))
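; Cannon projectile that costs the player a life on hit and is destroyed, passing over bonus objects and destroying itself on anything else.
; Mirror redirect functions, not called within this Blueprint, swap the velocity's X and Y and apply it in local space.
; The left turn negates the new Y and skips a repeat of the last left mirror hit, while the right turn has no such guard.
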(event OnComponentHit(Gfx)
  (params (HitComponent :type Primitive%20Component%20Object%20Reference) (OtherActor :type Actor%20Object%20Reference) (OtherComp :type Primitive%20Component%20Object%20Reference) (NormalImpulse :type Vector :default "0, 0, 0") (Hit :type Hit%20Result%20Structure%20%28by%20ref%29))
  (bind _asbp_player (Utilities|Casting|CastToBP_Player OtherActor)
    (:then
      (Default|DecrementLife _asbp_player)
      (Actor|DestroyActor))
    (:CastFailed
      (Utilities|Casting|CastToBonusObject OtherActor
        (:CastFailed
          (Actor|DestroyActor))))))

(event EventBeginPlay)

(fn ConstructionScript)

(fn SetVelocitytoLeft
  (params (MirorLeft :type BP%20Mirror%20Left%20Object%20Reference))
  (bind _projectilemovement (Variables|Default|GetProjectileMovement))
  (bind _velocity (Variables|/Script/Engine.MovementComponent|GetVelocity _projectilemovement))
  (if (not (== MirorLeft (Variables|Default|GetLastMirorLeftHit)))
    (Game|Components|ProjectileMovement|SetVelocityinLocalSpace _projectilemovement (Math|Vector|MakeVector (.y _velocity) (* (.x _velocity) -1.0) (.z _velocity)))
    (Variables|Default|SetLastMirorLeftHit MirorLeft)))

(fn SetVelocitytoRight
  (params (Velocity :type Vector))
  (Game|Components|ProjectileMovement|SetVelocityinLocalSpace (Variables|Default|GetProjectileMovement) (Math|Vector|MakeVector (.y Velocity) (.x Velocity) (.z Velocity))))
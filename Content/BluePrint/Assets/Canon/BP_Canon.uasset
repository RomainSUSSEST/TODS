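; BP_Canon is an automatic cannon actor that spawns projectiles at a fixed interval.
; Tick counts down a delay seeded from FireInterval on BeginPlay, then adds the interval back and calls Fire, carrying over any overshoot.
; Fire spawns the ProjectileToSpawn class at the root component's world location and rotation with unit scale.
; A debug "Hello" string prints after each shot.
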(event EventBeginPlay
  ;[1 1 1] Initialisation
  (Variables|Default|SetDelaiToFire (Variables|Default|GetFireInterval)))

(event Collision|EventActorBeginOverlap
  (params (OtherActor :type Actor%20Object%20Reference)))

(event EventTick
  (params (DeltaSeconds :type Float%20%28single-precision%29))
  ;[1 1 1] Update
  (if (> (Variables|Default|GetDelaiToFire) 0.0)
    (Variables|Default|SetDelaiToFire (- (Variables|Default|GetDelaiToFire) DeltaSeconds))
    (else
      (Variables|Default|SetDelaiToFire (+ (Variables|Default|GetDelaiToFire) (Variables|Default|GetFireInterval)))
      (CallFunction|Fire)
      (Development|PrintString "Hello"))))

(fn ConstructionScript)

(fn Fire
  (bind _defaultsceneroot (Variables|Default|GetDefaultSceneRoot))
  ;[1 1 1] Instantiate Projectile
  (Game|SpawnActorfromClass (Variables|Default|GetProjectileToSpawn) (Math|Transform|MakeTransform (Transformation|GetWorldLocation _defaultsceneroot) (Transformation|GetWorldRotation _defaultsceneroot)) "Undefined" 0 0))